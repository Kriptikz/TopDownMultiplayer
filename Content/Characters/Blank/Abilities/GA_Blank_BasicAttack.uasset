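; Gameplay Ability for the Blank character's basic attack, activated by a gameplay event that carries target data.
; On activation it stores the hit actor from the first target data entry, prints a debug message and ends after a short delay.
; The attack itself fires in OnEndAbility, which calls Attack on the BP_Character avatar with that target only if the owner has the State.Attack tag.
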(event `self.K2_OnEndAbility`
  (params (bWasCancelled :type Boolean))
  (if (`GameplayTagAssetInterface.HasMatchingGameplayTag` (`self.GetAbilitySystemComponentFromActorInfo` self) (struct :`TagName` "State.Attack"))
    (bind _asbp_character (cast `/Game/Blueprints/BP_Character` (`self.GetAvatarActorFromActorInfo`)))
    (`/Game/Blueprints/BP_Character.Attack` _asbp_character (`self.Target`))))

(event `self.K2_ActivateAbilityFromEvent`
  (params (EventData :type "GameplayEventData Structure (by ref)"))
  (set `self.Target` (`.HitActor` (`GameplayStatics.BreakHitResult` (`AbilitySystemBlueprintLibrary.GetHitResultFromTargetData` (`.TargetData` (break `GameplayEventData` EventData))))))
  (`KismetSystemLibrary.PrintString` "Basic Attack Activated" true true (struct :`R` 1.0 :`G` 0.990346 :`A` 1.0) 1.0)
  (`AbilityTask_WaitDelay.WaitDelay` 0.8
    (:`OnFinish`
      (`self.K2_EndAbility`))))