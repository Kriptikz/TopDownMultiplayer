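; Gameplay ability for the player's click command, choosing move, attack or use from what is under the cursor.
; An instant WaitTargetData with a cursor target actor feeds floor, attackable and usable checks that call BP_Character.
; Floor clicks always update TargetLocation, but call MoveToLocation only when the MoveToLocation tag is absent.
; An older MoveToTarget-based version remains, unconnected.
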(event `self.K2_ActivateAbility`
  ;[1 1 1] Determine our target
  (bind _returnvalue (`self.K2_CommitAbility`))
  (if _returnvalue
    (bind (_asynctaskproxy _data) (`AbilityTask_WaitTargetData.WaitTargetData` "None" "Instant" "/Script/TopDownMultiplayer.GameplayAbilityTargetActor_CursorTargetData" (struct) (struct) null)
      (:`ValidData`
        (bind _output (`|GetArrayItem` (`AbilitySystemBlueprintLibrary.GetActorsFromTargetData` _data)))
        (`/Engine/EditorBlueprintResources/StandardMacros.IsValid` _output
          (:`Is Valid`
            ;;[1 1 1] Floor
            (bind _returnvalue_2 (message `TargetableInterface.IsFloor` _output))
            (if _returnvalue_2
              (bind _asbp_character (cast `/Game/Blueprints/BP_Character` (`self.GetOwningActorFromActorInfo`)))
              (set `TDMCharacter.TargetLocation` (`AbilitySystemBlueprintLibrary.GetTargetDataEndPoint` _data) _asbp_character)
              (bind _returnvalue_3 (message `GameplayTagAssetInterface.HasMatchingGameplayTag` (`self.GetAbilitySystemComponentFromActorInfo`) (struct :`TagName` "Ability.Movement.MoveToLocation")))
              (if (not _returnvalue_3)
                (`/Game/Blueprints/BP_Character.MoveToLocation` _asbp_character))
              (else
                ;;[1 1 1] Attackable
                (bind _returnvalue_4 (message `TargetableInterface.IsAttackable` _output))
                (if _returnvalue_4
                  (bind _asbp_character_2 (cast `/Game/Blueprints/BP_Character` (`self.GetOwningActorFromActorInfo`))
                    (:`then`
                      (`/Game/Blueprints/BP_Character.Attack` _asbp_character_2))
                    (:`CastFailed`
                      _))
                  (else
                    ;;[1 1 1] Usable
                    (bind _returnvalue_5 (message `TargetableInterface.IsUsable` _output))
                    (if _returnvalue_5
                      (bind _asbp_character_3 (cast `/Game/Blueprints/BP_Character` (`self.GetOwningActorFromActorInfo`))
                        (:`then`
                          (`/Game/Blueprints/BP_Character.Use` _asbp_character_3))
                        (:`CastFailed`
                          _))))))))))
      (:`Cancelled`
        _))
    (`self.K2_EndAbility`)))