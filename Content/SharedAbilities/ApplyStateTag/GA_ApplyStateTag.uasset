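; GA_ApplyStateTag is a shared, event-triggered Gameplay Ability that applies a state tag effect to its owner.
; On activation it checks the event data's TargetTags for an exact Attack, Move or Idle state tag, in that priority order.
; The first match applies the corresponding GameplayEffect to the owner and ends the ability.
; With no match, the graph applies nothing and does not call EndAbility.
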(event `self.K2_ActivateAbilityFromEvent`
  (params (EventData :type "GameplayEventData Structure (by ref)"))
  (bind (_eventtag _instigator _target _optionalobject _optionalobject2 _contexthandle _instigatortags _targettags) (break `GameplayEventData` EventData))
  (if (`BlueprintGameplayTagLibrary.HasTag` _targettags (struct :`TagName` "State.Attack") true)
    (`self.BP_ApplyGameplayEffectToOwner` "/Game/SharedAbilities/ApplyStateTag/GE_AttackStateTag.GE_AttackStateTag_C")
    (`self.K2_EndAbility` :!label _label)
    (elif (`BlueprintGameplayTagLibrary.HasTag` _targettags (struct :`TagName` "State.Move") true)
      (`self.BP_ApplyGameplayEffectToOwner` "/Game/SharedAbilities/ApplyStateTag/GE_MoveStateTag.GE_MoveStateTag_C")
      (goto _label)
      (elif (`BlueprintGameplayTagLibrary.HasTag` _targettags (struct :`TagName` "State.Idle") true)
        (`self.BP_ApplyGameplayEffectToOwner` "/Game/SharedAbilities/ApplyStateTag/GE_IdleStateTag.GE_IdleStateTag_C")
        (goto _label)))))