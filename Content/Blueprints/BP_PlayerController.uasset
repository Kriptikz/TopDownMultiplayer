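; Player controller for click-to-move play, where the possessed camera pawn commands a separate AI-driven character.
; While move click is held, Tick sends cursor location and hovered actor to a server event that picks move, attack or use via floor, attackable and usable checks.
; Stop and three ability inputs likewise forward through server events to the pawn's controlled character or its AI.
; Local controllers also add a debug widget on BeginPlay.
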(event `self.ReceiveBeginPlay`
  ;[1 1 1] Add Debug View
  (if (`self.IsLocalPlayerController`)
    (bind _returnvalue (`|CreateWidget` "/Game/UI/WBP_DebugInfo.WBP_DebugInfo_C"))
    (`UserWidget.AddToViewport` _returnvalue 0)))

(event `self.ReceiveTick`
  (params (DeltaSeconds :type "Float (single-precision)"))
  ;[1 1 1] Tick
  (if (`self.IsPlayerMoveClickPressed`)
    (`self.ServerProcessPlayerMoveClick` (`self.CursorAimLocation`) (`self.HoveredActor`))))

(event `InputAction|Stop`
  (params (Key :type "Key Structure"))
  ;[0.05306 0 1] Inputs
  (:`Pressed`
    (set `self.IsPlayerMoveClickPressed` false)
    (`self.ServerProcessInputStop`)))

(event `InputAction|Ability1`
  (params (Key :type "Key Structure"))
  ;[0.05306 0 1] Inputs
  (:`Pressed`
    (`self.ServerProcessAbility1` (`self.CursorAimLocation`) (`self.HoveredActor`))))

(event `InputAction|Ability2`
  (params (Key :type "Key Structure"))
  ;[0.05306 0 1] Inputs
  (:`Pressed`
    (`self.ServerProcessAbility2` (`self.CursorAimLocation`) (`self.HoveredActor`))))

(event `InputAction|Player Move Click`
  (params (Key :type "Key Structure"))
  ;[0.05306 0 1] Inputs
  (:`Pressed`
    (set `self.IsPlayerMoveClickPressed` true))
  (:`Released`
    (set `self.IsPlayerMoveClickPressed` false)))

(event `InputAction|Ability3`
  (params (Key :type "Key Structure"))
  ;[0.05306 0 1] Inputs
  (:`Pressed`
    (`self.ServerProccessAbility3` (`self.CursorAimLocation`) (`self.HoveredActor`))))

(event `ServerProcessInputStop`
  ;[0.9768 1 0] Process Inputs
  (bind _asbp_player_camera_pawn (cast `/Game/Blueprints/BP_PlayerCameraPawn` (`self.K2_GetPawn`)))
  (`self.StopMovement` (`/Game/Blueprints/BP_PlayerCameraPawn.ControlledCharacterAI` _asbp_player_camera_pawn)))

(event `ServerProcessPlayerMoveClick`
  (params (AimLocation :type "Vector Structure") (HoveredActor :type "Actor Object Reference"))
  ;[0.9768 1 0] Process Inputs
  (`/Engine/EditorBlueprintResources/StandardMacros.IsValid` HoveredActor
    (:`Is Valid`
      (bind _returnvalue (message `TargetableInterface.IsFloor` HoveredActor))
      (if _returnvalue
        (bind _asbp_player_camera_pawn (cast `/Game/Blueprints/BP_PlayerCameraPawn` (`self.K2_GetPawn`)))
        (`/Game/Blueprints/BP_Character.MoveToLocation` (`/Game/Blueprints/BP_PlayerCameraPawn.ControlledCharacter` _asbp_player_camera_pawn) AimLocation)
        (else
          (bind _returnvalue_2 (message `TargetableInterface.IsAttackable` HoveredActor))
          (if _returnvalue_2
            (bind _asbp_player_camera_pawn_2 (cast `/Game/Blueprints/BP_PlayerCameraPawn` (`self.K2_GetPawn`)))
            (`/Game/Blueprints/BP_Character.Attack` (`/Game/Blueprints/BP_PlayerCameraPawn.ControlledCharacter` _asbp_player_camera_pawn_2) HoveredActor)
            (else
              (bind _returnvalue_3 (message `TargetableInterface.IsUsable` HoveredActor))
              (if _returnvalue_3
                (bind _asbp_player_camera_pawn_3 (cast `/Game/Blueprints/BP_PlayerCameraPawn` (`self.K2_GetPawn`)))
                (`/Game/Blueprints/BP_Character.Use` (`/Game/Blueprints/BP_PlayerCameraPawn.ControlledCharacter` _asbp_player_camera_pawn_3) HoveredActor)))))))))

(event `ServerProcessAbility1`
  (params (TargetLocation :type "Vector Structure") (TargetActor :type "Actor Object Reference"))
  ;[0.9768 1 0] Process Inputs
  (bind _asbp_player_camera_pawn (cast `/Game/Blueprints/BP_PlayerCameraPawn` (`self.K2_GetPawn`)))
  (`/Game/Blueprints/BP_Character.ActivateAbility1` (`/Game/Blueprints/BP_PlayerCameraPawn.ControlledCharacter` _asbp_player_camera_pawn) TargetLocation TargetActor))

(event `ServerProcessAbility2`
  (params (TargetLocation :type "Vector Structure") (TargetActor :type "Actor Object Reference"))
  ;[0.9768 1 0] Process Inputs
  (bind _asbp_player_camera_pawn (cast `/Game/Blueprints/BP_PlayerCameraPawn` (`self.K2_GetPawn`)))
  (`/Game/Blueprints/BP_Character.ActivateAbility2` (`/Game/Blueprints/BP_PlayerCameraPawn.ControlledCharacter` _asbp_player_camera_pawn) TargetLocation TargetActor))

(event `ServerProccessAbility3`
  (params (TargetLocation :type "Vector Structure") (TargetActor :type "Actor Object Reference"))
  ;[0.9768 1 0] Process Inputs
  (bind _asbp_player_camera_pawn (cast `/Game/Blueprints/BP_PlayerCameraPawn` (`self.K2_GetPawn`)))
  (`/Game/Blueprints/BP_Character.ActivateAbility3` (`/Game/Blueprints/BP_PlayerCameraPawn.ControlledCharacter` _asbp_player_camera_pawn) TargetLocation TargetActor))

(fn `UserConstructionScript`)