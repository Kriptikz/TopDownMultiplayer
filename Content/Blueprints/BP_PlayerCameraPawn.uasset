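; BP_PlayerCameraPawn is a player camera pawn that is separate from the character it is paired with.
; On BeginPlay, the authority spawns a BP_Blank and a TDMAIController at the pawn's transform, then has the controller possess the character.
; While Center Camera is held, Tick moves the pawn halfway toward that character's full transform each frame, a frame-rate-dependent smoothing.
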(event `self.ReceiveBeginPlay`
  (bind _returnvalue (`self.GetTransform`))
  (`/Engine/EditorBlueprintResources/ActorMacros.Switch Has Authority`
    (:`Authority`
      (bind _returnvalue_2 (`|SpawnActorFromClass` "/Game/Characters/Blank/BP_Blank.BP_Blank_C" _returnvalue "Undefined" "OverrideRootScale" null null))
      (set `self.ControlledCharacter` _returnvalue_2)
      (bind _returnvalue_3 (`|SpawnActorFromClass` "/Script/TopDownMultiplayer.TDMAIController" _returnvalue "Undefined" "OverrideRootScale" null null))
      (bind _output_get (set `self.ControlledCharacterAI` _returnvalue_3))
      (`Controller.Possess` _output_get (`self.ControlledCharacter`)))))

(event `self.ReceiveTick`
  (params (DeltaSeconds :type "Float (single-precision)"))
  (bind _controlledcharacter (`self.ControlledCharacter`))
  (if (`self.IsLockedCam`)
    (`/Engine/EditorBlueprintResources/StandardMacros.IsValid` _controlledcharacter
      (:`Is Valid`
        (`self.K2_SetActorTransform` (`KismetMathLibrary.TLerp` (`self.GetTransform` _controlledcharacter) (`self.GetTransform`) 0.5))))))

(event `InputAction|Center Camera`
  (params (Key :type "Key Structure"))
  (:`Pressed`
    (set `self.IsLockedCam` true))
  (:`Released`
    (set `self.IsLockedCam` false)))

(fn `UserConstructionScript`)