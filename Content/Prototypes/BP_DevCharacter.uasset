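; BP_DevCharacter is a prototype player character that tests Gameplay Ability System movement and team tags.
; Input activates the move-to-target ability or team A/B tag abilities, and a debug key prints which team tags it has.
; On becoming view target, it spawns a separate BP_DevPlayerCamera, links it to itself and blends the controller's view to it.
; The Center Camera input locks that camera while held.
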(event `self.ReceiveTick`
  (params (DeltaSeconds :type "Float (single-precision)"))
  (`parent.ReceiveTick` DeltaSeconds))

(event `InputAction|MoveAbility`
  (params (Key :type "Key Structure"))
  (:`Pressed`
    (`AbilitySystemComponent.TryActivateAbilityByClass` (`self.AbilitySystem`) "/Game/BaseAbilities/GA_MoveToTarget.GA_MoveToTarget_C" true)))

(event `Key|E`
  (params (Key :type "Key Structure"))
  (:`Pressed`
    (`AbilitySystemComponent.TryActivateAbilityByClass` (`self.AbilitySystem`) "/Game/BaseAbilities/ApplyTeamTags/GA_ApplyTeamATag.GA_ApplyTeamATag_C" true)))

(event `Key|G`
  (params (Key :type "Key Structure"))
  (bind _abilitysystem (`self.AbilitySystem`))
  (:`Pressed`
    (`|ExecutionSequence`
      (:`then_0`
        (if (`GameplayTagAssetInterface.HasMatchingGameplayTag` _abilitysystem (struct :`TagName` "Team.B"))
          (`KismetSystemLibrary.PrintString` "Has B Tag")))
      (:`then_1`
        (if (`GameplayTagAssetInterface.HasMatchingGameplayTag` _abilitysystem (struct :`TagName` "Team.A"))
          (`KismetSystemLibrary.PrintString` "Has A Tag"))))))

(event `Key|R`
  (params (Key :type "Key Structure"))
  (:`Pressed`
    (`AbilitySystemComponent.TryActivateAbilityByClass` (`self.AbilitySystem`) "/Game/BaseAbilities/ApplyTeamTags/GA_ApplyTeamBTag.GA_ApplyTeamBTag_C" true)))

(event `self.K2_OnBecomeViewTarget`
  (params (PC :type "PlayerController Object Reference"))
  (bind _asbp_dev_player_controller (cast `/Game/Prototypes/BP_DevPlayerController` PC))
  (bind _returnvalue (`|SpawnActorFromClass` "/Game/Prototypes/BP_DevPlayerCamera.BP_DevPlayerCamera_C" (`KismetMathLibrary.Conv_VectorToTransform` (`self.K2_GetActorLocation`)) "Undefined" "OverrideRootScale" _asbp_dev_player_controller null))
  (bind _output_get (set `self.PlayerCameraRef_0` _returnvalue))
  (set `/Game/Prototypes/BP_DevPlayerCamera.CharacterReference` self _output_get)
  (`PlayerController.SetViewTargetWithBlend` _asbp_dev_player_controller _returnvalue 0.0 "VTBlend_Linear" 0.0 false))

(event `InputAction|Center Camera`
  (params (Key :type "Key Structure"))
  (bind _playercameraref_0 (`self.PlayerCameraRef_0`))
  (:`Pressed`
    (set `/Game/Prototypes/BP_DevPlayerCamera.bIsLockedCamera` true _playercameraref_0))
  (:`Released`
    (set `/Game/Prototypes/BP_DevPlayerCamera.bIsLockedCamera` false _playercameraref_0)))

(fn `UserConstructionScript`
  (`parent.UserConstructionScript`))